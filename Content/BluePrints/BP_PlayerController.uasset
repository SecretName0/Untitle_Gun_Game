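; Player controller Blueprint that handles movement, looking, jumping and camera zoom for the BP_Player character.
; On BeginPlay it casts the controlled pawn to BP_Player and stores it for the input events to drive.
; Axis inputs move the character along its forward and right vectors and add sensitivity-scaled yaw and pitch to the controller.
; Zoom actions step the character's spring arm length in or out within a clamped range.
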(event EventBeginPlay
  (bind _asbp_player (Utilities|Casting|CastToBP_Player (Pawn|GetControlledPawn)))
  (Variables|플레이중인캐릭터|Set플레이어%20캐릭터 _asbp_player))

(event Input|ActionEvents|InputActionJumping(점프)
  (params (Key :type Key%20Structure :default "None"))
  ;[1 1 1] 캐릭터 움직임 관련
  ;;[1 1 1] 점프
  (:Pressed
    (Character|Jump (Variables|플레이중인캐릭터|Get플레이어%20캐릭터))))

(event Input|ActionEvents|InputAction카메라거리조절(가깝게)
  (params (Key :type Key%20Structure :default "None"))
  ;[1 1 1] 카메라 거리 조절
  (:Pressed
    (Variables|/Script/Engine.SpringArmComponent|SetTargetArmLength (Variables|/Game/BluePrints/BP_Player.BP_Player_C|GetSpringArm (Variables|플레이중인캐릭터|Get플레이어%20캐릭터)) (Math|Float|Clamp(Float) (- (Variables|/Script/Engine.SpringArmComponent|GetTargetArmLength (Variables|/Game/BluePrints/BP_Player.BP_Player_C|GetSpringArm (Variables|플레이중인캐릭터|Get플레이어%20캐릭터))) (Variables|Default|Get타깃%20암%20거리%20조절)) 3e+02 8e+02))))

(event Input|ActionEvents|InputAction카메라거리조절(멀게)
  (params (Key :type Key%20Structure :default "None"))
  ;[1 1 1] 카메라 거리 조절
  (:Pressed
    (Variables|/Script/Engine.SpringArmComponent|SetTargetArmLength (Variables|/Game/BluePrints/BP_Player.BP_Player_C|GetSpringArm (Variables|플레이중인캐릭터|Get플레이어%20캐릭터)) (Math|Float|Clamp(Float) (+ (Variables|/Script/Engine.SpringArmComponent|GetTargetArmLength (Variables|/Game/BluePrints/BP_Player.BP_Player_C|GetSpringArm (Variables|플레이중인캐릭터|Get플레이어%20캐릭터))) (Variables|Default|Get타깃%20암%20거리%20조절)) 3e+02 8e+02))))

(event Input|AxisEvents|InputAxisForward/Back
  (params (AxisValue :type Float%20%28single-precision%29))
  (bind _플레이어_캐릭터 (Variables|플레이중인캐릭터|Get플레이어%20캐릭터))
  ;[1 1 1] 캐릭터 움직임 관련
  ;;[1 1 1] 전후방 이동
  (Pawn|Input|AddMovementInput _플레이어_캐릭터 (Transformation|GetActorForwardVector _플레이어_캐릭터) AxisValue false))

(event Input|AxisEvents|InputAxisLeft/Right
  (params (AxisValue :type Float%20%28single-precision%29))
  (bind _플레이어_캐릭터 (Variables|플레이중인캐릭터|Get플레이어%20캐릭터))
  ;[1 1 1] 캐릭터 움직임 관련
  ;;[1 1 1] 좌우 이동
  (Pawn|Input|AddMovementInput _플레이어_캐릭터 (Transformation|GetActorRightVector _플레이어_캐릭터) AxisValue false))

(event Input|AxisEvents|InputAxisTurning
  (params (AxisValue :type Float%20%28single-precision%29))
  ;[1 1 1] 캐릭터 움직임 관련
  ;;[1 1 1] 캐릭터 회전
  (Class|PlayerController|AddYawInput (* AxisValue (Variables|민감도옵션|GetTurn%20Rate%28회전%20민감도%29))))

(event Input|AxisEvents|InputAxisLookUp/Down
  (params (AxisValue :type Float%20%28single-precision%29))
  ;[1 1 1] 캐릭터 움직임 관련
  ;;[1 1 1] 캐릭터 상하
  (Class|PlayerController|AddPitchInput (* AxisValue (Variables|민감도옵션|GetUp%20Down%20Rate%28상하%20민감도%29))))

(fn ConstructionScript)