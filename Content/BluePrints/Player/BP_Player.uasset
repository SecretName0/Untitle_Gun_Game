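; BP_Player is the player Blueprint, holding a Fire function for aiming and shooting a gun by line trace.
; Fire plays the fire montage, then deprojects the screen center and traces against object types to find the aim point.
; A second channel trace runs from the gun_head mesh socket to that point, correcting for camera-to-muzzle offset.
; Both traces draw debug lines, and the final hit result is unused.
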(fn ConstructionScript)

(fn Fire
  (bind _returnvalue (Viewport|GetViewportSize))
  (bind _returnvalue_2 (Game|GetPlayerController 0))
  (bind _returnvalue_3 (/ (.y _returnvalue) 2.0))
  (bind _returnvalue_4 (/ (.x _returnvalue) 2.0))
  (bind _returnvalue_5 (Math|Vector2D|MakeVector2D _returnvalue_4 _returnvalue_3))
  (bind (_worldposition _worlddirection _returnvalue_6) (Class|GameplayStatics|DeprojectScreentoWorld _returnvalue_2 _returnvalue_5))
  (Animation|PlayAnimMontage "/Game/Animations/Montage/AM_Fire.AM_Fire" 1.0 "start")
  (if _returnvalue_6
    (bind _outhit (Collision|LineTraceForObjects _worldposition (+ (* _worlddirection 5e+03) _worldposition) (Utilities|Array|MakeArray "ObjectTypeQuery1" "ObjectTypeQuery3" "ObjectTypeQuery2") false 0 "ForDuration" true "(R=1.000000,G=0.000000,B=0.000000,A=1.000000)" "(R=0.000000,G=1.000000,B=0.000000,A=1.000000)" 1.0))
    (Collision|LineTraceByChannel (.location (Transformation|GetSocketTransform (Variables|Character|GetMesh) "gun_head" "RTS_World")) (.Location (Collision|BreakHitResult _outhit)) "TraceTypeQuery3" false 0 "ForDuration" true "(R=1.000000,G=0.000000,B=0.000000,A=1.000000)" "(R=0.000000,G=1.000000,B=0.000000,A=1.000000)" 1.0) ; 이름처럼 트레이스 채널을 골라줌
  ))